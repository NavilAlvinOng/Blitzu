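; BP_Ball is the ball in a ball game that characters pick up by touching it.
; When unowned, a sphere overlap with a BP_CharacterBase records that character as owner, calls its TakeBallPossesion and marks the ball owned.
; ChangeBallState sets the owned flag and shows the decal only while the ball is free.
; UpdateBallMessage passes text to BP_GameMode to print to all.
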(event OnComponentBeginOverlap(Sphere1)
  (params (OverlappedComponent :type Primitive%20Component%20Object%20Reference) (OtherActor :type Actor%20Object%20Reference) (OtherComp :type Primitive%20Component%20Object%20Reference) (OtherBodyIndex :type Integer) (bFromSweep :type Boolean) (SweepResult :type Hit%20Result%20Structure%20%28by%20ref%29))
  (if (not (Variables|Default|GetbOwned))
    (bind _asbp_character_base (Utilities|Casting|CastToBP_CharacterBase OtherActor))
    (Variables|Default|SetballOwner _asbp_character_base)
    (Default|TakeBallPossesion _asbp_character_base self)
    (CallFunction|ChangeBallState true)))

(event Custom|ChangeBallState
  (params (bOwned :type Boolean))
  (bind _output_get (Variables|Default|SetbOwned bOwned))
  (Rendering|SetVisibility (Variables|Default|GetDecal) (not _output_get) false))

(event Custom|UpdateBallMessage
  (params (text :type Text))
  (bind _asbp_game_mode (Utilities|Casting|CastToBP_GameMode (Game|GetGameMode)))
  (Default|PrintMessagetoAll _asbp_game_mode text))

(fn ConstructionScript)