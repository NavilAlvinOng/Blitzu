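; Base character for a team ball game, with stat-driven movement, team-coloured mesh and decal, and ball possession.
; A MoveStateChecker macro allows axis input only while MOVING.
; Taking the ball attaches it to the hand socket and shows the decal; losing it reverses both.
; A moving carrier overlapping another character puts both into COMBAT and starts a GameMode battle event, while state changes refresh a debug stats widget on authority.
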(event Custom|MoveCharUpDown
  (params (axis :type Float%20%28single-precision%29))
  (bind _charactermovement (Variables|Character|GetCharacterMovement))
  ;[1 1 1] Input Movement
  (Utilities|MoveStateChecker
    (:CanMove
      (Class|PawnMovementComponent|AddInputVector _charactermovement (Math|Vector|MakeVector (* (* axis (Math|Conversions|ToFloat(Integer) (.speed (Variables|Stats|GetcharStats)))) -1.0) 0.0 0.0) false))
    (:Cannot
      (Components|Movement|StopMovementImmediately _charactermovement))))

(event Custom|MoveCharLeftRIght
  (params (axis :type Float%20%28single-precision%29))
  (bind _charactermovement (Variables|Character|GetCharacterMovement))
  ;[1 1 1] Input Movement
  (Utilities|MoveStateChecker
    (:CanMove
      (Class|PawnMovementComponent|AddInputVector _charactermovement (Math|Vector|MakeVector 0.0 (* (* axis (Math|Conversions|ToFloat(Integer) (.speed (Variables|Stats|GetcharStats)))) -1.0) 0.0) false))
    (:Cannot
      (Components|Movement|StopMovementImmediately _charactermovement))))

(event Custom|CreateWidgetUI
  ;[1 1 1] Create Debug Widget
  (Variables|UI|GetstatsUI
    (:then)
    (:else
      (bind _returnvalue (AddComponent|AddWidgetComponent false (Math|Transform|MakeTransform "0, 0,-200.000000")))
      (Transformation|AttachComponentToComponent _returnvalue (Variables|Character|GetMesh) "None" "KeepRelative" "KeepRelative" "KeepRelative" true)
      (bind _aswbp_player_stats (Utilities|Casting|CastToWBP_PlayerStats (UserInterface|GetUserWidgetObject _returnvalue)))
      (Variables|UI|SetstatsUI _aswbp_player_stats))))

(event Custom|UpdateStateUI
  ;[1 1 1] ShowUI
  (bind _statsui (Variables|UI|GetstatsUI)
    (:then
      (Default|ChangeState _statsui (Variables|States|GetmoveState) (Variables|States|GetplayState)))
    (:else)))

(event Custom|PrintLog_Server
  (params (text :type Text))
  ;[1 1 1] Create Debug Widget
  (bind _asbp_game_mode (Utilities|Casting|CastToBP_GameMode (Game|GetGameMode)))
  (Default|PrintMessagetoAll _asbp_game_mode text))

(event Custom|SetupStats
  (params (charStats :type F%20Character%20Stats%20Structure))
  ;[1 1 1] Stats
  (bind _output_get (Variables|Stats|SetcharStats charStats))
  (Variables|/Script/Engine.CharacterMovementComponent|SetMaxWalkSpeed (Variables|Character|GetCharacterMovement) (* (.Speed (Utilities|Struct|BreakFCharacterStats _output_get)) 1e+01)))

(event Custom|ShowStatsUI
  ;[1 1 1] ShowUI
  (CallFunction|CreateWidgetUI)
  (Default|DisplayStats (Variables|UI|GetstatsUI) (Variables|Stats|GetcharStats)))

(event EventPossessed
  (params (NewController :type Controller%20Object%20Reference))
  ;[1 1 1] Base
  (bind _asbp_player_controller (Utilities|Casting|CastToBP_PlayerController NewController))
  (bind _output_get (Variables|Default|SetplayerControl _asbp_player_controller))
  (Variables|Stats|Setteam (.playerteam (Variables|/Game/Blueprint/Core/BP_PlayerController.BP_PlayerController_C|GetplayerInfo _output_get))))

(event EventUnpossessed
  (params (OldController :type Controller%20Object%20Reference))
  (bind _charactermovement (Variables|Character|GetCharacterMovement))
  ;[1 1 1] Base
  (Class|PawnMovementComponent|AddInputVector _charactermovement "0, 0, 0" true)
  (Components|Movement|StopMovementImmediately _charactermovement))

(event EventBeginPlay
  ;[1 1 1] Base
)

(fn ConstructionScript)

(event Custom|SetCharacterColor
  (bind _team (Variables|Stats|Getteam))
  ;[1 1 1] Visual
  (Rendering|Material|SetMaterial (Variables|Character|GetMesh) 0 (Utilities|Select :Index _team :NewEnumerator0 0 :NewEnumerator1 0 :NewEnumerator2 "/Engine/MapTemplates/Materials/BasicAsset01.BasicAsset01"))
  (Rendering|Components|Decal|SetDecalMaterial (Variables|Default|GetDecal) (Utilities|Select :Index _team :NewEnumerator0 0 :NewEnumerator1 "/Game/Assets/Material/M_TeamA_Decal.M_TeamA_Decal" :NewEnumerator2 "/Game/Assets/Material/M_TeamB_Decal.M_TeamB_Decal")))

(event OnComponentBeginOverlap(Sphere)
  (params (OverlappedComponent :type Primitive%20Component%20Object%20Reference) (OtherActor :type Actor%20Object%20Reference) (OtherComp :type Primitive%20Component%20Object%20Reference) (OtherBodyIndex :type Integer) (bFromSweep :type Boolean) (SweepResult :type Hit%20Result%20Structure%20%28by%20ref%29))
  (if (and (Variables|Ball|GetbIsHoldingBall) (Utilities|Enum|Equal(Enum) (Variables|States|GetmoveState) "NewEnumerator0"))
    (bind _asbp_character_base (Utilities|Casting|CastToBP_CharacterBase OtherActor))
    (CallFunction|ChangePlayState _asbp_character_base "NewEnumerator2")
    (CallFunction|ChangePlayState "NewEnumerator3")
    (CallFunction|ChangeMoveState _asbp_character_base "NewEnumerator1")
    (CallFunction|ChangeMoveState "NewEnumerator1")
    (bind _asbp_game_mode (Utilities|Casting|CastToBP_GameMode (Game|GetGameMode)))
    (Default|StartBattleEvent _asbp_game_mode self _asbp_character_base)
    (Default|PrintMessagetoAll _asbp_game_mode "Battle Event has triggered!")))

(event Custom|ChangePlayState
  (params (playState :type EPlayState%20Enum :default "NewEnumerator0"))
  (Variables|States|SetplayState playState)
  (Networking|SwitchHasAuthority
    (:Authority
      (CallFunction|UpdateStateUI))))

(event Custom|ChangeMoveState
  (params (moveState :type EMovementState%20Enum :default "NewEnumerator0"))
  (Variables|States|SetmoveState moveState)
  (Networking|SwitchHasAuthority
    (:Authority
      (CallFunction|UpdateStateUI))))

(event Custom|TakeBallPossesion
  (params (ball :type BP%20Ball%20Object%20Reference))
  ;[1 1 1] Ball Attachments
  (if (not (Variables|Ball|GetbIsHoldingBall))
    (bind _output_get (Variables|Ball|Setball ball))
    (Variables|Ball|SetbIsHoldingBall true)
    (Transformation|AttachComponentToComponent _output_get (Variables|Character|GetMesh) "hand_r" "SnapToTarget" "SnapToTarget" "KeepRelative" true)
    (Rendering|SetVisibility (Variables|Default|GetDecal) true false)
    (CallFunction|PrintLogServer (Utilities|Text|FormatText "{i} grabbed the ball!" (Utilities|Struct|BreakFCharacterStats (Variables|Stats|GetcharStats))))))

(event Custom|LoseBallPossesion
  ;[1 1 1] Ball Attachments
  (if (Variables|Ball|GetbIsHoldingBall)
    (Variables|Ball|SetbIsHoldingBall false)
    (bind _ball (Variables|Ball|Getball)
      (:then
        (Transformation|DetachFromActor _ball "KeepWorld" "KeepWorld" "KeepWorld")
        (Variables|Ball|Setball 0)
        (Rendering|SetVisibility (Variables|Default|GetDecal) false false)
        (CallFunction|PrintLogServer (Utilities|Text|FormatText "{i} loses the ball!" (Utilities|Struct|BreakFCharacterStats (Variables|Stats|GetcharStats)))))
      (:else))))