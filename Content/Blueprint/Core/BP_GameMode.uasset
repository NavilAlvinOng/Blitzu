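; Game mode for a two-team ball game that spawns teams, starts the match and referees battles between two characters.
; On login, players get a debug team, characters from GameInstance team data at tagged PlayerStarts, and possession of the first.
; After a short delay it initializes HUDs, teams and debug stats.
; Battles await both choices: a match favors the attacker, otherwise the defender takes the ball, then state resets.
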(event Custom|StartTheGame
  ;[1 1 1] Start game
  (for _array_element (Variables|Default|GetplayerControllerList)
    (Default|InitHUD _array_element)
    (switch Utilities|FlowControl|Switch|SwitchonETeam (.playerteam (Variables|/Game/Blueprint/Core/BP_PlayerController.BP_PlayerController_C|GetplayerInfo _array_element))
      (:NewEnumerator1
        (Default|InitTeam _array_element (Variables|Team|GetteamAMembers)))
      (:NewEnumerator2
        (Default|InitTeam _array_element (Variables|Team|GetteamBMembers)))))
  (CallFunction|ShowAllDebugUI)
  (CallFunction|GetBallInfo))

(event Custom|LaunchGame
  ;[1 1 1] Start game
)

(event Custom|GetBallInfo
  (bind _outactors (Actor|GetAllActorsOfClass "/Game/Blueprint/BallGame/BP_Ball.BP_Ball_C"))
  (Variables|Default|SetballRef (Utilities|Array|Get(acopy) _outactors)))

(event Custom|SpawnPlayer
  (params (playerController :type BP%20Player%20Controller%20Object%20Reference))
  (bind _playerinfo (Variables|/Game/Blueprint/Core/BP_PlayerController.BP_PlayerController_C|GetplayerInfo playerController))
  (bind _giref (Variables|Default|GetGIRef)
    (:then
      _)
    (:else
      (bind _asbp_game_instance (Utilities|Casting|CastToBP_GameInstance (Game|GetGameInstance)))
      (Variables|Default|SetGIRef _asbp_game_instance)))
  (for (_array_element _array_index) (Default|GetTeamInfo _giref (.playerteam _playerinfo))
    (bind _returnvalue (Game|SpawnActorfromClass "/Game/Blueprint/Character/BP_CharacterBase.BP_CharacterBase_C" (Spawn|ReturnSpawnPoint (.playerteam _playerinfo) _array_index) "Undefined" 0 (.playerteam _playerinfo) 0))
    (Networking|SwitchHasAuthority
      (:Authority
        (Default|SetupStats _returnvalue _array_element)
        (if (== _array_index 0)
          (Pawn|Possess playerController _returnvalue))
        (switch Utilities|FlowControl|Switch|SwitchonETeam (.playerteam _playerinfo)
          (:NewEnumerator1
            (Utilities|Array|Add (Variables|Team|GetteamAMembers) _returnvalue))
          (:NewEnumerator2
            (Utilities|Array|Add (Variables|Team|GetteamBMembers) _returnvalue)))))))

(event Custom|StartGame_Server
  ;[1 1 1] Start game
  (CallFunction|StarttheGame))

(event Custom|ResetBattleEvent
  (Variables|Combat|SetattackerChoice "NewEnumerator0")
  (Variables|Combat|SetdefenderChoice "NewEnumerator0")
  (Variables|Combat|Setatker 0)
  (Variables|Combat|Setdfender 0))

(event Custom|PrintMessageToAll
  (params (text :type Text))
  (for _array_element (Variables|Default|GetplayerControllerList)
    (Default|PrintSystemMessage _array_element text)))

(event Custom|ShowAllDebugUI
  (Utilities|FlowControl|Sequence
    (:then_0
      (for _array_element (Variables|Team|GetteamAMembers)
        (Default|ShowStatsUI _array_element)))
    (:then_1
      (for _array_element_2 (Variables|Team|GetteamBMembers)
        (Default|ShowStatsUI _array_element_2)))))

(event Custom|StartBattleEvent
  (params (attacker :type BP%20Character%20Base%20Object%20Reference) (defender :type BP%20Character%20Base%20Object%20Reference))
  (bind _output_get (Variables|Combat|Setatker attacker))
  (bind _output_get_2 (Variables|Combat|Setdfender defender))
  (Utilities|FlowControl|Sequence
    (:then_0
      (bind _asbp_player_controller (Utilities|Casting|CastToBP_PlayerController (Pawn|GetController _output_get)))
      (Default|EngageBattle _asbp_player_controller))
    (:then_1
      (bind _asbp_player_controller_2 (Utilities|Casting|CastToBP_PlayerController (Pawn|GetController _output_get_2)))
      (Default|EngageBattle _asbp_player_controller_2))))

(event Custom|LogChoice
  (params (state :type EPlayState%20Enum :default "NewEnumerator0") (choice :type EDirection%20Enum :default "NewEnumerator0"))
  (Development|PrintString (Utilities|String|Append (Utilities|String|EnumtoString state) " choice is " (Utilities|String|EnumtoString choice)) true true "(R=1.000000,G=0.035682,B=0.000000,A=1.000000)" 5.0)
  (switch Utilities|FlowControl|Switch|SwitchonEPlayState state
    (:NewEnumerator2
      (Variables|Combat|SetdefenderChoice choice))
    (:NewEnumerator3
      (Variables|Combat|SetattackerChoice choice)))
  (CallFunction|CheckCombatResult))

(event Custom|CheckCombatResult
  (bind _atker (Variables|Combat|Getatker))
  (if (and (Utilities|Enum|NotEqual(Enum) (Variables|Combat|GetdefenderChoice) "NewEnumerator0") (Utilities|Enum|NotEqual(Enum) (Variables|Combat|GetattackerChoice) "NewEnumerator0"))
    (bind _winner (CallFunction|CalculateBattleResult))
    (CallFunction|PrintMessagetoAll (Utilities|Text|ToText(String) (Utilities|String|Append "Winner is " (Utilities|String|ToString(Text) (.charactername (Variables|/Game/Blueprint/Character/BP_CharacterBase.BP_CharacterBase_C|GetcharStats _winner))) "!")))
    (Default|ChangeMoveState _atker "NewEnumerator0")
    (Utilities|FlowControl|Sequence
      (:then_0
        (bind _asbp_player_controller (Utilities|Casting|CastToBP_PlayerController (Pawn|GetController _atker)))
        (Default|EndBattle _asbp_player_controller))
      (:then_1
        (bind _asbp_player_controller_2 (Utilities|Casting|CastToBP_PlayerController (Pawn|GetController (Variables|Combat|Getdfender))))
        (Default|EndBattle _asbp_player_controller_2))
      (:then_2
        (CallFunction|ResetBattleEvent)))))

(event EventPostLogin
  (params (NewPlayer :type Player%20Controller%20Object%20Reference))
  (Spawn|InitSpawnPoints)
  (Networking|SwitchHasAuthority
    (:Authority
      (bind _asbp_player_controller (Utilities|Casting|CastToBP_PlayerController NewPlayer))
      (bind _returnvalue (Utilities|Array|Add (Variables|Default|GetplayerControllerList) _asbp_player_controller))
      (|DEBUGSETTEAM _asbp_player_controller _returnvalue)
      (CallFunction|SpawnPlayer _asbp_player_controller))))

(event EventBeginPlay
  (Spawn|InitSpawnPoints)
  (bind _asbp_game_instance (Utilities|Casting|CastToBP_GameInstance (Game|GetGameInstance)))
  (Variables|Default|SetGIRef _asbp_game_instance)
  (Utilities|FlowControl|Delay 2.0)
  (Networking|SwitchHasAuthority
    (:Authority
      (CallFunction|StarttheGame))
    (:Remote
      (CallFunction|StartGameServer))))

(fn ConstructionScript)

(fn InitSpawnPoints
  (bind _spawnpoints_a (Variables|Spawn|GetspawnPoints_A))
  (if (not (Utilities|Array|IsValidIndex _spawnpoints_a))
    (Utilities|Array|Clear _spawnpoints_a)
    (Utilities|Array|Clear (Variables|Spawn|GetspawnPoints_B))
    (bind _outactors (Actor|GetAllActorsOfClass "/Script/Engine.PlayerStart"))
    (bind _output_get (LocalVariables|SetallPlayerStarts _outactors))
    (for _array_element _output_get
      (if (Utilities|Name|Equal(Name) (Variables|/Script/Engine.PlayerStart|GetPlayerStartTag _array_element) (Utilities|String|StringToName (CallFunction|EzGetText "TEAM_A_ID")))
        (Utilities|Array|Add (Variables|Spawn|GetspawnPoints_A) _array_element)
        (elif (Utilities|Name|Equal(Name) (Variables|/Script/Engine.PlayerStart|GetPlayerStartTag _array_element) (Utilities|String|StringToName (CallFunction|EzGetText "TEAM_B_ID")))
          (Utilities|Array|Add (Variables|Spawn|GetspawnPoints_B) _array_element))))))

(fn ReturnSpawnPoint
  (params (team :type ETeam%20Enum :default "NewEnumerator0") (index :type Integer))
  (switch Utilities|FlowControl|Switch|SwitchonETeam team
    (:NewEnumerator0
      _)
    (:NewEnumerator1
      (LocalVariables|Settemp (Variables|Spawn|GetspawnPoints_A)))
    (:NewEnumerator2
      (LocalVariables|Settemp (Variables|Spawn|GetspawnPoints_B))))
  (return (Transformation|GetActorTransform (Utilities|Array|Get(acopy) (LocalVariables|Gettemp) index))))

(fn CalculateBattleResult
  (bind _dfender (Variables|Combat|Getdfender))
  (if (== (Variables|Combat|GetattackerChoice) (Variables|Combat|GetdefenderChoice))
    (Development|PrintString "Attacker WINS!")
    (return (Variables|Combat|Getatker))
    (else
      (Development|PrintString "Defender WINS!")
      (Default|LoseBallPossesion (Variables|Combat|Getatker))
      (Default|TakeBallPossesion _dfender (Variables|Default|GetballRef))
      (return _dfender))))