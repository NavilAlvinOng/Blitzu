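; Player controller for a team of characters, forwarding movement input to the possessed pawn and cycling possession through the team on Tab.
; Team setup stores the pawns, initializes their color and stats UI on authority, and sets their move state.
; Battle events switch the camera manager between combat and normal cameras and show or remove a choice widget, with decisions logged through the game mode.
; It also creates the HUD and relays system messages to it.
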(event Custom|SendDecisionToServer
  (params (state :type EPlayState%20Enum :default "NewEnumerator0") (choice :type EDirection%20Enum :default "NewEnumerator0"))
  ;[1 1 1] Combat
  (bind _asbp_game_mode (Utilities|Casting|CastToBP_GameMode (Game|GetGameMode)))
  (Default|LogChoice _asbp_game_mode state choice))

(event Custom|InitTeam
  (params (team :type Array%20of%20BP%20Character%20Base%20Object%20References))
  ;[1 1 1] Initialization
  (Variables|Default|SetteamPawn team)
  (for _array_element team
    (Networking|SwitchHasAuthority
      (:Authority
        (Default|SetCharacterColor _array_element)
        (Default|ShowStatsUI _array_element))))
  (CallFunction|StartPlayer))

(event Custom|StartPlayer
  ;[1 1 1] Initialization
  (for _array_element (Variables|Default|GetteamPawn)
    (Default|ChangeMoveState _array_element "NewEnumerator0")))

(event Custom|SwapChar
  (bind _teampawn (Variables|Default|GetteamPawn))
  ;[1 1 1] Swap to next Character
  (if (>= (+ (Variables|Default|GetcurrentPossesed) 1) (Utilities|Array|Length _teampawn))
    (Variables|Default|SetcurrentPossesed 0)
    (else
      (Variables|Default|SetcurrentPossesed (+ (Variables|Default|GetcurrentPossesed) 1))))
  (Pawn|UnPossess)
  (Pawn|Possess (Utilities|Array|Get(acopy) _teampawn (Variables|Default|GetcurrentPossesed))))

(event Custom|EngageBattle
  ;[1 1 1] Combat
  (bind _asbp_camera_manager (Utilities|Casting|CastToBP_CameraManager (Game|GetPlayerCameraManager 0)))
  (Default|ToCombatCamera _asbp_camera_manager)
  (bind _returnvalue (UserInterface|CreateWidget "/Game/UI/Widgets/WBP_BattleChoice.WBP_BattleChoice_C" self))
  (UserInterface|Viewport|AddtoViewport _returnvalue 0)
  (Default|SetupUI _returnvalue (Variables|/Game/Blueprint/Character/BP_CharacterBase.BP_CharacterBase_C|GetplayState (Variables|Default|GetcontrolledPawn)))
  (Variables|Default|SetchoiceUI _returnvalue))

(event Custom|EndBattle
  ;[1 1 1] Combat
  (bind _asbp_camera_manager (Utilities|Casting|CastToBP_CameraManager (Game|GetPlayerCameraManager 0)))
  (Default|ToNormalCamera _asbp_camera_manager)
  (bind _choiceui (Variables|Default|GetchoiceUI)
    (:then
      (Widget|RemovefromParent _choiceui))
    (:else)))

(event EventPossess
  (params (PossessedPawn :type Pawn%20Object%20Reference))
  ;[1 1 1] Possession
  (bind _asbp_character_base (Utilities|Casting|CastToBP_CharacterBase PossessedPawn))
  (Variables|Default|SetcontrolledPawn _asbp_character_base))

(fn ConstructionScript)

(event Input|ActionEvents|InputActionActionUp
  (params (Key :type Key%20Structure :default "None"))
  ;[1 1 1] Input
)

(event Input|ActionEvents|InputActionActionTab
  (params (Key :type Key%20Structure :default "None"))
  ;[1 1 1] Input
  (:Pressed
    (CallFunction|SwapChar)))

(event Input|ActionEvents|InputActionActionLeft
  (params (Key :type Key%20Structure :default "None"))
  ;[1 1 1] Input
)

(event Input|ActionEvents|InputActionActionRight
  (params (Key :type Key%20Structure :default "None"))
  ;[1 1 1] Input
)

(event Input|ActionEvents|InputActionActionDown
  (params (Key :type Key%20Structure :default "None"))
  ;[1 1 1] Input
)

(event Input|AxisEvents|InputAxisMoveForward
  (params (AxisValue :type Float%20%28single-precision%29))
  ;[1 1 1] Input
  (bind _controlledpawn (Variables|Default|GetcontrolledPawn)
    (:then
      (Default|MoveCharUpDown _controlledpawn AxisValue))
    (:else)))

(event Input|AxisEvents|InputAxisMoveRight
  (params (AxisValue :type Float%20%28single-precision%29))
  ;[1 1 1] Input
  (bind _controlledpawn (Variables|Default|GetcontrolledPawn)
    (:then
      (Default|MoveCharLeftRIght _controlledpawn AxisValue))
    (:else)))

(event Custom|InitHUD
  ;[1 1 1] UI
  (bind _returnvalue (UserInterface|CreateWidget "/Game/UI/Widgets/WBP_GameHUd.WBP_GameHud_C" (Game|GetPlayerController 0)))
  (Variables|Default|Sethud _returnvalue)
  (UserInterface|Viewport|AddtoViewport _returnvalue 0))

(event Custom|PrintSystemMessage
  (params (text :type Text))
  ;[1 1 1] UI
  (bind _hud (Variables|Default|Gethud)
    (:then
      (Default|ShowMessage _hud text))
    (:else)))