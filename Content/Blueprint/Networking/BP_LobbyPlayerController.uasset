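; Player controller for the home menu and multiplayer lobby that creates the menu UI and relays session requests.
; InitHUD shows the home menu outside a lobby, or a host or client lobby menu depending on network authority.
; Host and destroy-lobby events delegate to a lazily cached BP_GameInstance, while DestroyLobbySession destroys the session directly and returns to MainMenu on success.
; MoveLevel is an empty stub.
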(event Custom|MoveLevel
  (params (levelName :type String)))

(event Custom|DestroyLobbySession
  (|DestroySession (Game|GetPlayerController 0)
    (:OnSuccess
      (Game|OpenLevel(byName) "MainMenu"))))

(event Custom|ServerHostLobby
  ;[1 1 1] Server Host Lobby
  (bind _gameinstance_ (Variables|Default|GetgameInstance_)
    (:then
      _)
    (:else
      (CallFunction|SetupGameInstance)))
  (Default|InstanceHostLobby _gameinstance_ self))

(event Custom|InitHUD
  (bind _self self)
  ;[1 1 1] Init HUD
  (bind _gameinstance_ (Variables|Default|GetgameInstance_)
    (:then
      _)
    (:else
      (CallFunction|SetupGameInstance)))
  (if (Variables|/Game/Blueprint/Core/BP_GameInstance.BP_GameInstance_C|GetbIsInLobby_ _gameinstance_)
    (Networking|SwitchHasAuthority
      (:Authority
        (bind _returnvalue (UserInterface|CreateWidget "/Game/UI/Widgets/Networking/WBP_LobbyHostMenu.WBP_LobbyHostMenu_C" 0 _self))
        (UserInterface|Viewport|AddtoViewport _returnvalue 0))
      (:Remote
        (bind _returnvalue_2 (UserInterface|CreateWidget "/Game/UI/Widgets/Networking/WBP_LobbyClientMenu.WBP_LobbyClientMenu_C" _self _self))
        (UserInterface|Viewport|AddtoViewport _returnvalue_2 0)))
    (else
      (bind _returnvalue_3 (UserInterface|CreateWidget "/Game/UI/Widgets/Networking/WBP_HomeMenu.WBP_HomeMenu_C" _self))
      (UserInterface|Viewport|AddtoViewport _returnvalue_3 0))))

(event Custom|SetupGameInstance
  ;[1 1 1] Setup Game Instance
  (bind _asbp_game_instance (Utilities|Casting|CastToBP_GameInstance (Game|GetGameInstance)))
  (Variables|Default|SetgameInstance_ _asbp_game_instance))

(event Custom|ServerDestroyLobby
  (bind _gameinstance_ (Variables|Default|GetgameInstance_)
    (:then
      _)
    (:else
      (CallFunction|SetupGameInstance)))
  (Default|InstanceDestroyLobby _gameinstance_ self))

(event EventBeginPlay)

(fn ConstructionScript)