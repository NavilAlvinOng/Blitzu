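; Player camera manager that switches the view between a normal and a combat camera.
; Two events toggle a Combat flag, which selects either the normal offset and rotation or the combat transform.
; The BlueprintUpdateCamera override places the camera at the target's location plus that world-space offset, with absolute rotation and fixed FOV, switching instantly without blending.
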(event Custom|ToCombatCamera
  (Variables|Default|SetbCombat true))

(event Custom|ToNormalCamera
  (Variables|Default|SetbCombat false))

(fn ConstructionScript)

(fn BlueprintUpdateCamera
  (params (CameraTarget :type Actor%20Object%20Reference))
  (bind _combattransform (Variables|Default|GetcombatTransform))
  (bind _bcombat (Variables|Default|GetbCombat))
  (|CallParentFunction CameraTarget)
  (return (+ (Transformation|GetActorLocation CameraTarget) (select _bcombat (.location _combattransform) (Variables|Default|GetCameraOffset))) (select _bcombat (.rotation _combattransform) (Variables|Default|GetcameraRotOffset)) 9e+01 true))